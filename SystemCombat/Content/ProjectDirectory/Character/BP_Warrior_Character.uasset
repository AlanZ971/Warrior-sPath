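; BP_Warrior_Character is the player-controlled warrior, with movement, camera look and an early light attack.
; BeginPlay registers the warrior Enhanced Input mapping context, and movement follows the controller's yaw.
; Light attack input sets the LightATK flag between press and completion.
; Light_AttackTrigger overlaps only print hit or fail by casting to BP_Enemy, without checking that flag; the Guard section is empty.
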(event `self.ReceiveBeginPlay`
  (bind _asplayer_controller (cast `PlayerController` (`self.GetController`)))
  (bind _output_get (set `self.Player Controller` _asplayer_controller))
  (bind _returnvalue (pcsubsystem `EnhancedInputLocalPlayerSubsystem` _output_get))
  (`/Engine/EditorBlueprintResources/StandardMacros.IsValid` _returnvalue
    (:`Is Valid`
      (`EnhancedInputSubsystemInterface.AddMappingContext` _returnvalue "/Game/ProjectDirectory/Input_Mapping/WarriorMappingContext.WarriorMappingContext" 0 (struct)))))

(event `EnhancedInput|/Game/ProjectDirectory/Input_Mapping/Actions/IA_Movement`
  (params (ActionValue :type "Vector2D Structure") (ElapsedSeconds :type "Float (double-precision)") (TriggeredSeconds :type "Float (double-precision)") (InputAction :type "InputAction Object Reference" :default "/Game/ProjectDirectory/Input_Mapping/Actions/IA_Movement.IA_Movement"))
  (bind (_returnvalue_roll _returnvalue_pitch _returnvalue_yaw) (`KismetMathLibrary.BreakRotator` (`self.GetControlRotation`)))
  (bind (_returnvalue_roll_2 _returnvalue_pitch_2 _returnvalue_yaw_2) (`KismetMathLibrary.BreakRotator` (`self.GetControlRotation`)))
  ;[0 0.5052 0.1081] Movement
  (:`Triggered`
    (`self.AddMovementInput` (`KismetMathLibrary.GetRightVector` (`KismetMathLibrary.MakeRotator` _returnvalue_roll_2 0.0 _returnvalue_yaw_2)) ActionValue_X)
    (`self.AddMovementInput` (`KismetMathLibrary.GetForwardVector` (`KismetMathLibrary.MakeRotator` 0.0 0.0 _returnvalue_yaw)) ActionValue_Y)))

(event `EnhancedInput|/Game/ProjectDirectory/Input_Mapping/Actions/IA_Guard`
  (params (ActionValue :type Boolean) (ElapsedSeconds :type "Float (double-precision)") (TriggeredSeconds :type "Float (double-precision)") (InputAction :type "InputAction Object Reference" :default "/Game/ProjectDirectory/Input_Mapping/Actions/IA_Guard.IA_Guard"))
  ;[0 0 0] Guard
)

(event `EnhancedInput|/Game/ProjectDirectory/Input_Mapping/Actions/IA_Parry`
  (params (ActionValue :type Boolean) (ElapsedSeconds :type "Float (double-precision)") (TriggeredSeconds :type "Float (double-precision)") (InputAction :type "InputAction Object Reference" :default "/Game/ProjectDirectory/Input_Mapping/Actions/IA_Parry.IA_Parry"))
  ;[0 0 0] Guard
)

(event `EnhancedInput|/Game/ProjectDirectory/Input_Mapping/Actions/IA_Look`
  (params (ActionValue :type "Vector2D Structure") (ElapsedSeconds :type "Float (double-precision)") (TriggeredSeconds :type "Float (double-precision)") (InputAction :type "InputAction Object Reference" :default "/Game/ProjectDirectory/Input_Mapping/Actions/IA_Look.IA_Look"))
  ;[0 0.5052 0.1081] Camera
  (:`Triggered`
    (`self.AddControllerYawInput` ActionValue_X)
    (`self.AddControllerPitchInput` ActionValue_Y)))

(event `EnhancedInput|/Game/ProjectDirectory/Input_Mapping/Actions/IA_Light_Attack`
  (params (ActionValue :type Boolean) (ElapsedSeconds :type "Float (double-precision)") (TriggeredSeconds :type "Float (double-precision)") (InputAction :type "InputAction Object Reference" :default "/Game/ProjectDirectory/Input_Mapping/Actions/IA_Light_Attack.IA_Light_Attack"))
  ;[1 0 0.06069] Attack
  (:`Started`
    (set `self.Light_ATK?` true))
  (:`Completed`
    (set `self.Light_ATK?` false)))

(event `EnhancedInput|/Game/ProjectDirectory/Input_Mapping/Actions/IA_Heavy_Attack`
  (params (ActionValue :type Boolean) (ElapsedSeconds :type "Float (double-precision)") (TriggeredSeconds :type "Float (double-precision)") (InputAction :type "InputAction Object Reference" :default "/Game/ProjectDirectory/Input_Mapping/Actions/IA_Heavy_Attack.IA_Heavy_Attack"))
  ;[1 0 0.06069] Attack
)

(event `self.Light_AttackTrigger.OnComponentBeginOverlap`
  (params (OverlappedComponent :type "PrimitiveComponent Object Reference") (OtherActor :type "Actor Object Reference") (OtherComp :type "PrimitiveComponent Object Reference") (OtherBodyIndex :type Integer) (bFromSweep :type Boolean) (SweepResult :type "HitResult Structure (by ref)"))
  (cast `/Game/ProjectDirectory/Character/BP_Enemy` OtherActor
    (:`then`
      (`KismetSystemLibrary.PrintString` "Light hit"))
    (:`CastFailed`
      (`KismetSystemLibrary.PrintString` "Light Failed"))))

(fn `UserConstructionScript`)
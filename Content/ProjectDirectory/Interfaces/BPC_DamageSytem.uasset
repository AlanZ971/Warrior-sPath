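; Damage system component that tracks a character's health, blocking and death, and reports results through OnBlocked, OnDamageResponse and OnDeath calls.
; TakeDamageComp routes hits through CanBeDamaged to ignore, block or apply them.
; Blocked hits reduce damage, drain a gauge scaled by damage (more if unparriable), and re-enter TakeDamageComp with zero damage to trigger the reaction.
; A looping timer from Initialize ends blocking once the gauge empties.
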(event `Initialize`
  (params (Character :type "Character Object Reference"))
  (set `self.Character` Character)
  (`KismetSystemLibrary.K2_SetTimerDelegate` (delegate `CheckShield`) 0.1 true))

(event `CheckShield`
  (if (<= (`self.CurrentBlockGauge`) 0.0)
    (set `self.IsBlocking` false)))

(fn `Block_Energy`
  (params (AmmountDmg :type "Float (double-precision)") (CanBeParried :type Boolean))
  (bind _returnvalue (- (`self.CurrentBlockGauge`) (* (+ (/ AmmountDmg 50.0) 1.0) (`self.Base Gauge Substract`))))
  (if CanBeParried
    (set `self.CurrentBlockGauge` _returnvalue)
    (else
      (set `self.CurrentBlockGauge` (- _returnvalue 20.0))
      (`KismetSystemLibrary.PrintString` "Unblockable")))
  (return))

(fn `Take_DamageComp`
  (params (DamageInfos :type "/Game/ProjectDirectory/Interfaces/DamageSytem/S_DamageInfos Structure"))
  (returns (`WasDamaged?` :type Boolean))
  (bind (_dmg_ammount _dmg_reaction _canbeblocked _canbeparried) (break `/Game/ProjectDirectory/Interfaces/DamageSytem/S_DamageInfos` DamageInfos))
  (`self.CanBeDamaged` _canbeblocked _canbeparried ; Vérifie le typed de dégats
    (:`IgnoreDamage`
      (`KismetSystemLibrary.PrintString` "Ignored")
      (return false))
    (:`BlockDamage`
      (if (not (<= (`self.CurrentBlockGauge`) 0.0))
        (bind _output_get (set `self.Health` (- (`self.Health`) (* _dmg_ammount (`self.Reduction_DegatsBlock`)))))
        (if (not (<= _output_get 0.0))
          (`self.Block_Energy` _dmg_ammount _canbeparried) ; Calcul de la vie blocké et réduction gauge de dégats
          (`self.Take_DamageComp` (make `/Game/ProjectDirectory/Interfaces/DamageSytem/S_DamageInfos` 0.0 "NewEnumerator3"))
          (`self.On Blocked` _canbeblocked)
          (return true)
          (else
            (set `self.IsDead?` true :!label _label)
            (`self.On Death`)))
        (else
          (bind _output_get_2 (set `self.Health` (- (`self.Health`) _dmg_ammount) :!label _label_2))
          (if (<= _output_get_2 0.0)
            (goto _label)
            (else
              (`self.On damage response` _dmg_reaction))))))
    (:`DoDamage`
      (goto _label_2)))
  (return true))
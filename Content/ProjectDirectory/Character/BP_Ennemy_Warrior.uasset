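; Enemy warrior character with sword combat, carrying player-style input bindings plus a timer that auto-triggers light attacks when flagged as Attacker.
; Montage-driven light combo deals damage through a sphere trace; heavy attack hits a trigger's overlaps after a timed delay.
; BPCDamageSytem handles health and blocking, feeding back hit reactions, stagger, stun, parry and ragdoll death.
; Polling timers drive the parry window, shield visibility and delayed block-gauge regeneration.
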(event `EnhancedInput|/Game/ProjectDirectory/Input_Mapping/Actions/IA_Movement`
  (params (ActionValue :type "Vector2D Structure") (ElapsedSeconds :type "Float (double-precision)") (TriggeredSeconds :type "Float (double-precision)") (InputAction :type "InputAction Object Reference" :default "/Game/ProjectDirectory/Input_Mapping/Actions/IA_Movement.IA_Movement"))
  (bind (_returnvalue_roll _returnvalue_pitch _returnvalue_yaw) (`KismetMathLibrary.BreakRotator` (`self.GetControlRotation`)))
  (bind (_returnvalue_roll_2 _returnvalue_pitch_2 _returnvalue_yaw_2) (`KismetMathLibrary.BreakRotator` (`self.GetControlRotation`)))
  ;[0 0.5052 0.1081] Movement
  (:`Triggered`
    (`self.AddMovementInput` (`KismetMathLibrary.GetRightVector` (`KismetMathLibrary.MakeRotator` _returnvalue_roll_2 0.0 _returnvalue_yaw_2)) ActionValue_X)
    (`self.AddMovementInput` (`KismetMathLibrary.GetForwardVector` (`KismetMathLibrary.MakeRotator` 0.0 0.0 _returnvalue_yaw)) ActionValue_Y)))

(event `EnhancedInput|/Game/ProjectDirectory/Input_Mapping/Actions/IA_Look`
  (params (ActionValue :type "Vector2D Structure") (ElapsedSeconds :type "Float (double-precision)") (TriggeredSeconds :type "Float (double-precision)") (InputAction :type "InputAction Object Reference" :default "/Game/ProjectDirectory/Input_Mapping/Actions/IA_Look.IA_Look"))
  ;[0 0.5052 0.1081] Camera
  (:`Triggered`
    (`self.AddControllerYawInput` ActionValue_X)
    (`self.AddControllerPitchInput` ActionValue_Y)))

(event `TimerATK`
  (if (`self.Attacker?`)
    (if (> (`self.Timer ATK`) 2.5)
      (`KismetSystemLibrary.K2_SetTimerDelegate` (delegate `TimerATK`) 0.0)
      (`self.Select atk`)
      (set `self.Timer ATK` 0.0)
      (else
        (set `self.Timer ATK` (+ (`self.Timer ATK`) (`self.Delta Second` 1.0)))))))

(event `self.ReceiveBeginPlay`
  (bind _returnvalue (`|CreateWidget` "/Game/ProjectDirectory/UI/W_HealthBar.W_HealthBar_C" null self null null null))
  (`WidgetComponent.SetWidget` (`self.Health_Bar`) _returnvalue)
  (set `self.CurrTimerRegen` 0.0)
  (`KismetSystemLibrary.K2_SetTimer` null "DetectBlock?" 0.1 true)
  (`/Game/ProjectDirectory/Interfaces/BPC_DamageSytem.Initialize` (`self.BPC_DamageSytem`) self)
  (`SceneComponent.SetVisibility` (`self.Shield`) false false)
  (`KismetSystemLibrary.K2_SetTimerDelegate` (delegate `ShieldUp`) 0.1 true)
  (`KismetSystemLibrary.K2_SetTimerDelegate` (delegate `TimerATK`) 0.01 true))

(event `Select atk`
  (if (not (`self.Attacking?`)) :!label _label
    (`|PlayMontage` (`self.Mesh`) (select `int` (`self.LightATKCombo`) :`0` "/Game/ProjectDirectory/CharaDesign/Animation/GreatSWord/Knight/LightATK/Great_Sword_Slash1_Montage.Great_Sword_Slash1_Montage" :`1` "/Game/ProjectDirectory/CharaDesign/Animation/GreatSWord/Knight/LightATK/Great_Sword_Slash2_Montage.Great_Sword_Slash2_Montage" :`2` "/Game/ProjectDirectory/CharaDesign/Animation/GreatSWord/Knight/LightATK/Great_Sword_Slash3_Montage.Great_Sword_Slash3_Montage" :!type "AnimMontage Object Reference")
      (:`then`
        (`/Engine/EditorBlueprintResources/StandardMacros.IncrementInt` (`self.LightATKCombo`)
          (:`  `
            (if (>= (`self.LightATKCombo`) 2)
              (set `self.LightATKCombo` 0)
              (`KismetSystemLibrary.K2_SetTimer` null "TimerAnimLightATK" 0.01 true)
              (set `self.Attacking?` true)
              (set `self.SwordTraceON` false)
              (`self.Dissable Inputs` :!label _label_2)))))
      (:`OnInterrupted`
        (set `self.Attacking?` false)))))

(event `EnhancedInput|/Game/ProjectDirectory/Input_Mapping/Actions/IA_Guard`
  (params (ActionValue :type Boolean) (ElapsedSeconds :type "Float (double-precision)") (TriggeredSeconds :type "Float (double-precision)") (InputAction :type "InputAction Object Reference" :default "/Game/ProjectDirectory/Input_Mapping/Actions/IA_Guard.IA_Guard"))
  (bind _bpc_damagesytem (`self.BPC_DamageSytem`))
  ;[0 0.5274 1] Guard
  (:`Started`
    (set `/Game/ProjectDirectory/Interfaces/BPC_DamageSytem.IsBlocking` true _bpc_damagesytem)
    (set `self.ParryON` true)
    (`KismetSystemLibrary.K2_SetTimer` null "TimingParry" 0.01 true)
    (set `self.TimerParry` 0.0)
    (`SceneComponent.SetVisibility` (`self.Shield`) true false))
  (:`Completed`
    (set `/Game/ProjectDirectory/Interfaces/BPC_DamageSytem.IsBlocking` false _bpc_damagesytem)))

(event `ShieldUp`
  (bind _shield (`self.Shield`))
  (if (`/Game/ProjectDirectory/Interfaces/BPC_DamageSytem.IsBlocking` (`self.BPC_DamageSytem`))
    (`SceneComponent.SetVisibility` _shield true false)
    (else
      (`SceneComponent.SetVisibility` _shield false false))))

(event `EnhancedInput|/Game/ProjectDirectory/Input_Mapping/Actions/IA_Light_Attack`
  (params (ActionValue :type Boolean) (ElapsedSeconds :type "Float (double-precision)") (TriggeredSeconds :type "Float (double-precision)") (InputAction :type "InputAction Object Reference" :default "/Game/ProjectDirectory/Input_Mapping/Actions/IA_Light_Attack.IA_Light_Attack"))
  ;[1 0 0.06069] Attack
  (:`Triggered`
    (goto _label)))

(event `EnhancedInput|/Game/ProjectDirectory/Input_Mapping/Actions/IA_Heavy_Attack`
  (params (ActionValue :type Boolean) (ElapsedSeconds :type "Float (double-precision)") (TriggeredSeconds :type "Float (double-precision)") (InputAction :type "InputAction Object Reference" :default "/Game/ProjectDirectory/Input_Mapping/Actions/IA_Heavy_Attack.IA_Heavy_Attack"))
  ;[1 0 0.06069] Attack
  (:`Triggered`
    (if (not (`self.Attacking?`))
      (`self.PlayAnimMontage` "/Game/ProjectDirectory/CharaDesign/Animation/GreatSWord/Knight/HeavyATK/HeavyATK_Montage.HeavyATK_Montage")
      (`KismetSystemLibrary.K2_SetTimer` null "TimerAnimHeavyATK" 0.01 true)
      (set `self.Attacking?` true)
      (set `self.SwordTraceON` false)
      (goto _label_2))))

(event `TimingParry`
  ;[0 0.5274 1] Guard
  (if (>= (`self.TimerParry`) 0.5)
    (set `self.ParryON` false)
    (`KismetSystemLibrary.K2_SetTimerDelegate` (delegate `TimingParry`))
    (else
      (set `self.TimerParry` (+ (`self.TimerParry`) (* (`GameplayStatics.GetWorldDeltaSeconds`) 1.0))))))

(event `Death`
  (bind _mesh (`self.Mesh`))
  ;[0 0 0] States
  (`PrimitiveComponent.SetSimulatePhysics` _mesh true)
  (`PrimitiveComponent.SetCollisionEnabled` _mesh "QueryAndPhysics")
  (`self.DisableInput` (`GameplayStatics.GetPlayerController` 0)))

(event `TimerAnimLightATK`
  ;[1 1 1] Timer Animations
  (if (`self.Attacking?`)
    (if (`self.ActorHit?`)
      (`self.StopSwordNow`))
    (else
      (`self.StopSwordTrace` :!label _label_3)
      (`KismetSystemLibrary.K2_SetTimer` null "TimerATK" 0.01 true))))

(event `Blocked`
  (params (CanBeParied :type Boolean))
  ;[0 0 0] States
  (if (and CanBeParied (`self.ParryON`))
    (`self.PlayAnimMontage` "/Game/ProjectDirectory/CharaDesign/Animation/GreatSWord/Knight/BlockingTest/Actual_Parryreat_sword_Montage.Actual_Parryreat_sword_Montage")
    (else
      (`KismetSystemLibrary.PrintString` "Blocked?!")
      (`KismetSystemLibrary.K2_SetTimer` null "DetectBlock?" 0.1 true)
      (set `self.CurrTimerRegen` 0.0))))

(event `StopSwordNow`
  ;[1 1 1] Timer Animations
  (goto _label_3))

(event `TimerAnimHeavyATK`
  ;[1 1 1] Timer Animations
  (bind _output_get (set `self.TimerAnim` (+ (`self.TimerAnim`) (* (`GameplayStatics.GetWorldDeltaSeconds`) 1.0))))
  (if (>= _output_get 2.3)
    (message `/Game/ProjectDirectory/Interfaces/DamageSytem/BPI_DamageSystem.Take Damage` (`PrimitiveComponent.GetOverlappingActors` (`self.Heavy_AttackTrigger`) null) (make `/Game/ProjectDirectory/Interfaces/DamageSytem/S_DamageInfos` 25.0 "NewEnumerator2"))
    (`KismetSystemLibrary.K2_SetTimerDelegate` (delegate `TimerAnimHeavyATK`))
    (`self.StopSwordTrace`)
    (`self.Enable Inputs`)
    (set `self.TimerAnim` 0.0)))

(event `Damage Response`
  (params (DmgResponse :type "/Game/ProjectDirectory/Interfaces/DamageSytem/E_DmgResponse Enum" :default "NewEnumerator0"))
  ;[0 0 0] States
  (switch `/Game/ProjectDirectory/Interfaces/DamageSytem/E_DmgResponse` DmgResponse
    (:`NewEnumerator1`
      (`self.PlayAnimMontage` "/Game/ProjectDirectory/CharaDesign/Animation/GreatSWord/Knight/Impact/Impact_NoBlock_1_Montage.Impact_NoBlock_1_Montage")
      (set `self.CurrTimerRegen` 0.0 :!label _label_4))
    (:`NewEnumerator2`
      (`self.PlayAnimMontage` "/Game/ProjectDirectory/CharaDesign/Animation/GreatSWord/Knight/Impact/Impact_NoBlock_2_Montage.Impact_NoBlock_2_Montage")
      (goto _label_4))
    (:`NewEnumerator3`
      (if (<= (`/Game/ProjectDirectory/Interfaces/BPC_DamageSytem.CurrentBlockGauge` (`self.BPC_DamageSytem`)) 0.0)
        (`KismetSystemLibrary.K2_SetTimerDelegate` (delegate `Stunned`) 0.1)
        (`KismetSystemLibrary.K2_SetTimer` null "TimerRegen" 0.01 true)
        (`KismetSystemLibrary.K2_SetTimer` null "BlockEnergyRegen" 0.0)
        (set `self.MaxTimerRegen` 2.0)))))

(event `Stunned`
  ;[0 0 0] States
  (`self.Dissable Inputs`)
  (set `self.Anim Stun` true)
  (`/Engine/EditorBlueprintResources/StandardMacros.DoOnce` false :!label _label_5
    (:`Completed`
      (`|PlayMontage` (`self.Mesh`) "/Game/ProjectDirectory/CharaDesign/Animation/GreatSWord/Knight/Stunned/Zombie_Reaction_Hit_Montage.Zombie_Reaction_Hit_Montage"
        (:`OnCompleted`
          (if (`self.Anim Stun`)
            (goto _label_5 :!via `Reset`)))))))

(fn `BlockEnergyRegen`
  (bind _bpc_damagesytem (`self.BPC_DamageSytem`))
  (bind _bpc_damagesytem_2 (`self.BPC_DamageSytem`))
  (bind _bpc_damagesytem_3 (`self.BPC_DamageSytem`))
  (if (< (`/Game/ProjectDirectory/Interfaces/BPC_DamageSytem.CurrentBlockGauge` (`self.BPC_DamageSytem`)) 0.0)
    (set `/Game/ProjectDirectory/Interfaces/BPC_DamageSytem.CurrentBlockGauge` 0.0 (`self.BPC_DamageSytem`)))
  (if (> (`/Game/ProjectDirectory/Interfaces/BPC_DamageSytem.CurrentBlockGauge` _bpc_damagesytem_3) (`/Game/ProjectDirectory/Interfaces/BPC_DamageSytem.MaxBlockGauge` _bpc_damagesytem_3))
    (set `/Game/ProjectDirectory/Interfaces/BPC_DamageSytem.CurrentBlockGauge` (`/Game/ProjectDirectory/Interfaces/BPC_DamageSytem.MaxBlockGauge` _bpc_damagesytem) _bpc_damagesytem)
    (`KismetSystemLibrary.K2_SetTimer` null "BlockEnergyRegen")
    (`KismetSystemLibrary.K2_SetTimer` null "DetectBlock?" 0.1 true)
    (set `self.Anim Stun` false)
    (else
      (set `/Game/ProjectDirectory/Interfaces/BPC_DamageSytem.CurrentBlockGauge` (+ (`/Game/ProjectDirectory/Interfaces/BPC_DamageSytem.CurrentBlockGauge` _bpc_damagesytem_2) (`self.Delta Second` 25.0)) _bpc_damagesytem_2))))

(fn `DetectBlock?`
  (bind _bpc_damagesytem (`self.BPC_DamageSytem`))
  (if (< (`/Game/ProjectDirectory/Interfaces/BPC_DamageSytem.CurrentBlockGauge` _bpc_damagesytem) (`/Game/ProjectDirectory/Interfaces/BPC_DamageSytem.MaxBlockGauge` _bpc_damagesytem))
    (`KismetSystemLibrary.K2_SetTimer` null "DetectBlock?")
    (`KismetSystemLibrary.K2_SetTimer` null "TimerRegen" 0.01 true)
    (set `self.MaxTimerRegen` 15.0)))

(fn `Get Current Block Gauge`
  (returns (CurrentBlockGauge :type "Float (double-precision)"))
  (return (`/Game/ProjectDirectory/Interfaces/BPC_DamageSytem.CurrentBlockGauge` (`self.BPC_DamageSytem`))))

(fn `Get current health`
  (returns (Health :type "Float (double-precision)"))
  (return (`/Game/ProjectDirectory/Interfaces/BPC_DamageSytem.Health` (`self.BPC_DamageSytem`))))

(fn `Get Max Block Gauge`
  (returns (MaxBlockgauge :type "Float (double-precision)"))
  (return (`/Game/ProjectDirectory/Interfaces/BPC_DamageSytem.MaxBlockGauge` (`self.BPC_DamageSytem`))))

(fn `Get max health`
  (returns (MaxHealth :type "Float (double-precision)"))
  (return (`/Game/ProjectDirectory/Interfaces/BPC_DamageSytem.MaxHealth` (`self.BPC_DamageSytem`))))

(fn `Sword Light LineTrace`
  (bind (_outhit _returnvalue) (`KismetSystemLibrary.SphereTraceSingle` :`Start` (`SceneComponent.K2_GetComponentLocation` (`self.PivotSword`)) :`End` (`SceneComponent.K2_GetComponentLocation` (`self.Sword_END`)) :`Radius` 25.0 :`TraceChannel` "TraceTypeQuery3" :`DrawDebugType` "ForDuration" :`DrawTime` 1.0))
  (if _returnvalue
    (set `self.ActorHit?` true)
    (message `/Game/ProjectDirectory/Interfaces/DamageSytem/BPI_DamageSystem.Take Damage` (`.HitActor` (`GameplayStatics.BreakHitResult` _outhit)) (make `/Game/ProjectDirectory/Interfaces/DamageSytem/S_DamageInfos` 10.0 "NewEnumerator1" true true))))

(fn `Take Damage`
  (params (DamageInfos :type "/Game/ProjectDirectory/Interfaces/DamageSytem/S_DamageInfos Structure"))
  (returns (WasDamaged :type Boolean))
  (bind _wasdamaged_ (`/Game/ProjectDirectory/Interfaces/BPC_DamageSytem.Take_DamageComp` (`self.BPC_DamageSytem`) DamageInfos))
  (return _wasdamaged_))

(fn `TimerRegen`
  (if (<= (`self.CurrTimerRegen`) (`self.MaxTimerRegen`))
    (set `self.CurrTimerRegen` (+ (`self.CurrTimerRegen`) (`self.Delta Second` 1.0)))
    (else
      (`KismetSystemLibrary.K2_SetTimer` null "TimerRegen")
      (`KismetSystemLibrary.K2_SetTimer` null "BlockEnergyRegen" 0.01 true)
      (set `self.CurrTimerRegen` 0.0))))

(fn `UserConstructionScript`
  (bind _bpc_damagesytem (`self.BPC_DamageSytem`))
  (add `/Game/ProjectDirectory/Interfaces/BPC_DamageSytem.On Death` _bpc_damagesytem (`|CreateDelegate` :!event `Death`))
  (add `/Game/ProjectDirectory/Interfaces/BPC_DamageSytem.On Blocked` _bpc_damagesytem (`|CreateDelegate` :!event `Blocked`))
  (add `/Game/ProjectDirectory/Interfaces/BPC_DamageSytem.On damage response` _bpc_damagesytem (`|CreateDelegate` :!event `Damage Response`)))
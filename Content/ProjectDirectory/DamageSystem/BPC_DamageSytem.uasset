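; Damage system component that tracks health and resolves incoming hits for the actor that owns it.
; TakeDamage passes DamageInfo flags to a Can be damaged macro, which routes each hit to block, damage or no damage based on death, invincibility and blocking.
; Event dispatchers announce blocks with parry eligibility, death at zero health, and damage responses for interruptible or forced-interrupt hits.
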(fn `Take_Damage`
  (params (Damage_Info :type "/Game/ProjectDirectory/DamageSystem/S_DamageInfo Structure"))
  (returns (`Was_Damaged?` :type Boolean))
  (bind (_ammoutdmg _damagetype _damageresponse _shoulddamageinvincible_ _canbeblocked_ _canbeparried_ _shouldforceinterrupt) (break `/Game/ProjectDirectory/DamageSystem/S_DamageInfo` Damage_Info))
  (`self.Can be damaged?` _shoulddamageinvincible_ _canbeblocked_
    (:`BlockDamage`
      (`self.OnBlocked` _canbeparried_)
      (return false))
    (:`DoDamage`
      (bind _output_get (set `self.Health` (- (`self.Health`) _ammoutdmg)))
      (if (<= _output_get 0.0)
        (set `self.IsDead?` true)
        (`self.OnDeath`)
        (return true)
        (elif (or (`self.Interruptible?`) _shouldforceinterrupt)
          (`self.Damage Response` _damageresponse)
          (return true))))
    (:`NoDamage`
      (`KismetSystemLibrary.PrintString` "NO DAMAGE")
      (return false))))